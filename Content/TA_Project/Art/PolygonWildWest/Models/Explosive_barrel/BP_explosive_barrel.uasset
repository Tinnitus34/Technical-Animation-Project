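; Explosive barrel actor that spawns a scaled explosion particle effect and destroys itself in its damage response; the blast applies no damage itself.
; The construction script binds to the BPCDamageSystem component's damage-response and death delegates, with the Death event left empty.
; Damage interface functions forward damage and death state to that component, report health and max health minus a fixed offset, and stub out healing.
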(event Custom|Death
  ;[0.15 0.15 0.15 0.5] Explosion effect
)

(event Custom|DamageResponse
  (params (NewParam :type E_DamageResponse%20Enum :default "NewEnumerator0") (NewParam2 :type Actor%20Object%20Reference))
  (bind _returnvalue (Transformation|GetActorLocation))
  ;[0.15 0.15 0.15 0.5] Explosion effect
  (Effects|SpawnEmitteratLocation "/Game/TA_Project/StarterContent/Particles/P_Explosion.P_Explosion" _returnvalue (Math|Conversions|RotationFromXVector _returnvalue) "2.000000,2.000000,1.000000")
  (Actor|DestroyActor))

(event EventBeginPlay)

(event Collision|EventActorBeginOverlap
  (params (OtherActor :type Actor%20Object%20Reference)))

(event EventTick
  (params (DeltaSeconds :type Float%20%28single-precision%29)))

(fn ConstructionScript
  (bind _bpc_damagesystem (Variables|Default|GetBPC_DamageSystem))
  (EventDispatchers|BindEventtoOnDeath _bpc_damagesystem (EventDispatchers|CreateEvent :!event Custom|Death))
  (EventDispatchers|BindEventtoOnDamageResponse _bpc_damagesystem (EventDispatchers|CreateEvent :!event Custom|DamageResponse)))

(fn GetCurrentHealth
  (return (- (Variables|/Game/TA_Project/Blueprints/Systems/DamageSystem/BPC_DamageSystem.BPC_DamageSystem_C|GetHealth (Variables|Default|GetBPC_DamageSystem)) 75.0)))

(fn GetMaxHealth
  (return (- (Variables|/Game/TA_Project/Blueprints/Systems/DamageSystem/BPC_DamageSystem.BPC_DamageSystem_C|GetMaxHealth (Variables|Default|GetBPC_DamageSystem)) 75.0)))

(fn GetTeamNumber
  (return 0))

(fn Heal
  (params (Amount :type Float%20%28double-precision%29))
  (return 0.0))

(fn IsDead
  (return (Variables|/Game/TA_Project/Blueprints/Systems/DamageSystem/BPC_DamageSystem.BPC_DamageSystem_C|GetIsDead (Variables|Default|GetBPC_DamageSystem))))

(fn TakeDamage
  (params (DamageInfo :type S%20Damage%20Info%20Structure) (Damage%20Causer :type Actor%20Object%20Reference))
  (bind _wasdamaged (Default|TakeDamage (Variables|Default|GetBPC_DamageSystem) DamageInfo Damage%20Causer))
  (return _wasdamaged))
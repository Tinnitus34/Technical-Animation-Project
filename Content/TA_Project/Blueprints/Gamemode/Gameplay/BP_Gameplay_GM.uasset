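; Game mode for a wave-based shooter that runs the start countdown, enemy waves, HUD and win/lose outcome.
; On BeginPlay it creates the HUD, configures WaveEnemySystem and starts a looping timer for the countdown to the first wave.
; Tick polls player ammo, death and wave completion to update the HUD, disabling input at game end.
; An intro-sequence path that hides the player exists but is disconnected from execution.
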(event Custom|Countdown
  (CallFunction|StartCountdown (stale EventBeginPlay _returnvalue)))

(event EventBeginPlay
  (|CallParentFunction)
  (CallFunction|DefineHUD)
  (Utilities|FlowControl|Delay (CallFunction|GetSequenceDuration))
  (Default|SetWaveParameters (Variables|Default|GetWaveEnemySystem) 10 10)
  (bind _returnvalue (Utilities|Time|SetTimerbyEvent (EventDispatchers|CreateEvent :!event Custom|Countdown) 1.0 true)))

(event EventTick
  (params (DeltaSeconds :type Float%20%28single-precision%29))
  (Utilities|FlowControl|Sequence
    (:then_0
      (CallFunction|UpdateAmmoCounter))
    (:then_1
      (CallFunction|EndGame))
    (:then_2
      (CallFunction|ShowPlayeronEndSequence))))

(event EventCallonEnemyDefeated
  (Default|OnEnemyDefeated (Variables|Default|GetWaveEnemySystem)))

(fn ConstructionScript
  (|CallParentFunction))

(fn StartCountdown
  (params (Handle :type Timer%20Handle%20Structure%20%28by%20ref%29))
  (bind _count (Variables|Default|GetCount))
  (Widget|SetVisibility (Variables|/Game/TA_Project/Blueprints/Systems/WaveSystem/WB_WavemodeHUD.WB_WavemodeHUD_C|GetText_StartingTime (Variables|Default|GetHUD)) "Visible")
  (Math|Integer|DecrementInt _count
    (:%20%20
      (Rendering|Components|TextRender|SetText (Variables|/Game/TA_Project/Blueprints/Systems/WaveSystem/WB_WavemodeHUD.WB_WavemodeHUD_C|GetText_StartingTime (Variables|Default|GetHUD)) (Utilities|Text|FormatText "Starting in: {Time} seconds" _count))
      (if (<= (Variables|Default|GetCount) 0)
        (Utilities|Time|ClearandInvalidateTimerbyHandle Handle)
        (Widget|SetVisibility (Variables|/Game/TA_Project/Blueprints/Systems/WaveSystem/WB_WavemodeHUD.WB_WavemodeHUD_C|GetText_StartingTime (Variables|Default|GetHUD)) "Hidden")
        (Default|NewWave (Variables|Default|GetWaveEnemySystem))
        (Widget|SetVisibility (Variables|/Game/TA_Project/Blueprints/Systems/WaveSystem/WB_WavemodeHUD.WB_WavemodeHUD_C|GetText_WaveNumber (Variables|Default|GetHUD)) "Visible")
        (Widget|SetVisibility (Variables|/Game/TA_Project/Blueprints/Systems/WaveSystem/WB_WavemodeHUD.WB_WavemodeHUD_C|GetText_KillsRemaining (Variables|Default|GetHUD)) "Visible")))))

(fn EndGame
  (bind _hud (Variables|Default|GetHUD))
  (bind _hud_2 (Variables|Default|GetHUD))
  (bind _dead (Class|BPIDamagable|IsDead(Message) (Game|GetPlayerCharacter 0)))
  (if _dead
    (Widget|SetVisibility (Variables|/Game/TA_Project/Blueprints/Systems/WaveSystem/WB_WavemodeHUD.WB_WavemodeHUD_C|GetText_WaveNumber _hud) "Collapsed")
    (Widget|SetVisibility (Variables|/Game/TA_Project/Blueprints/Systems/WaveSystem/WB_WavemodeHUD.WB_WavemodeHUD_C|GetText_KillsRemaining _hud) "Collapsed")
    (Rendering|Components|TextRender|SetText (Variables|/Game/TA_Project/Blueprints/Systems/WaveSystem/WB_WavemodeHUD.WB_WavemodeHUD_C|GetText_Win _hud) "YOU LOSE!")
    (Widget|SetVisibility (Variables|/Game/TA_Project/Blueprints/Systems/WaveSystem/WB_WavemodeHUD.WB_WavemodeHUD_C|GetText_Win _hud) "Visible")
    (Input|DisableInput (Game|GetPlayerController 0) 0)
    (elif (Variables|/Game/TA_Project/Blueprints/Systems/WaveSystem/BPC_WaveSystem.BPC_WaveSystem_C|GetIsGameEnded (Variables|Default|GetWaveEnemySystem))
      (Widget|SetVisibility (Variables|/Game/TA_Project/Blueprints/Systems/WaveSystem/WB_WavemodeHUD.WB_WavemodeHUD_C|GetText_WaveNumber _hud_2) "Collapsed")
      (Widget|SetVisibility (Variables|/Game/TA_Project/Blueprints/Systems/WaveSystem/WB_WavemodeHUD.WB_WavemodeHUD_C|GetText_KillsRemaining _hud_2) "Collapsed")
      (Rendering|Components|TextRender|SetText (Variables|/Game/TA_Project/Blueprints/Systems/WaveSystem/WB_WavemodeHUD.WB_WavemodeHUD_C|GetText_Win _hud_2) "YOU WIN!")
      (Widget|SetVisibility (Variables|/Game/TA_Project/Blueprints/Systems/WaveSystem/WB_WavemodeHUD.WB_WavemodeHUD_C|GetText_Win _hud_2) "Visible")
      (Input|DisableInput (Game|GetPlayerController 0) 0))))

(fn PlaySequenceandHidePlayer
  (Rendering|SetVisibility (Variables|/Script/Engine.Character|GetMesh (Game|GetPlayerCharacter 0)) false false)
  (Input|DisableInput (Game|GetPlayerController 0) 0)
  (bind _returnvalue (Sequencer|Player|CreateLevelSequencePlayer "/Game/TA_Project/Art/Sequence/Cowboy_CtrlRig_Take1.Cowboy_CtrlRig_Take1"))
  (bind _output_get (Variables|Default|SetSequencePlayer _returnvalue))
  (Sequencer|Player|Play _output_get :!class /Script/MovieScene.MovieSceneSequencePlayer))

(fn GetSequenceDuration
  (bind _sequenceplayer (Variables|Default|GetSequencePlayer)
    (:then
      (return (Math|Conversions|ToFloat(Integer) (/ (Class|MovieSceneSequencePlayer|GetFrameDuration _sequenceplayer) (.numerator (Class|MovieSceneSequencePlayer|GetFrameRate _sequenceplayer))))))
    (:else)))

(fn DefineHUD
  (bind _returnvalue (UserInterface|CreateWidget "/Game/TA_Project/Blueprints/Systems/WaveSystem/WB_WavemodeHUD.WB_WavemodeHUD_C" (Game|GetPlayerController 0)))
  (bind _output_get (Variables|Default|SetHUD _returnvalue))
  (UserInterface|Viewport|AddtoViewport _output_get 0))

(fn ShowPlayeronEndSequence
  (bind _sequenceplayer (Variables|Default|GetSequencePlayer))
  (Variables|Default|GetSequencePlayer
    (:then
      (if (>= (+ (.value (.frame (Sequencer|Player|GetCurrentTime _sequenceplayer))) 1) (Class|MovieSceneSequencePlayer|GetFrameDuration _sequenceplayer))
        (Utilities|FlowControl|DoOnce false
          (:Completed
            (Rendering|SetVisibility (Variables|/Script/Engine.Character|GetMesh (Game|GetPlayerCharacter 0)) true false)
            (Input|EnableInput (Game|GetPlayerController 0) 0)))))
    (:else)))

(fn UpdateAmmoCounter
  (bind (_ammovalue _carriedammovalue) (Class|BPIWeaponSystemCharacter|GetAmmoValues(Message) (Game|GetPlayerCharacter 0)))
  (Rendering|Components|TextRender|SetText (Variables|/Game/TA_Project/Blueprints/Systems/WaveSystem/WB_WavemodeHUD.WB_WavemodeHUD_C|GetText_Ammo (Variables|Default|GetHUD)) (Utilities|Text|FormatText "{ammo}/{carriedammo}" _ammovalue _carriedammovalue)))

(fn GetRefHUD
  (return (Variables|Default|GetHUD)))

(fn GetWaveEnemyComponent
  (return (Variables|Default|GetWaveEnemySystem)))
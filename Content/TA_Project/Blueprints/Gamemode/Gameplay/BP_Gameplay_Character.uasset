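; Playable gameplay character Blueprint that adds revolver hitscan shooting on top of its parent class.
; When the Shoot input starts while aiming, it plays the gunshot sound and runs a debug-drawn Visibility line trace forward from the camera.
; It sends a TakeDamage message to the hit actor, dealing triple damage when the hit bone is the head or neck.
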(event Input|EnhancedActionEvents|EnhancedInputActionIA_Shoot
  (params (ActionValue :type Boolean) (ElapsedSeconds :type Float%20%28double-precision%29) (TriggeredSeconds :type Float%20%28double-precision%29) (InputAction :type Input%20Action%20Object%20Reference :default "/Game/TA_Project/Blueprints/Input/Actions/IA_Shoot.IA_Shoot"))
  (bind _camera (Variables|Default|GetCamera))
  (bind _returnvalue (Transformation|GetWorldLocation _camera))
  ;[0.15 0.15 0.15 0.5] Shoot Input
  (:Started
    (if (Variables|Default|GetIsAiming)
      (Audio|PlaySound2D "/Game/TA_Project/Sounds/SoundEffects/RevolverShootSound.RevolverShootSound" 0.3 1.0 0.0 0 0)
      (bind (_outhit _returnvalue_2) (Collision|LineTraceByChannel _returnvalue (+ _returnvalue (* (Math|Vector|GetForwardVector _camera) 5e+03)) "TraceTypeQuery1" false 0 "ForDuration" true "(R=1.000000,G=0.000000,B=0.000000,A=1.000000)" "(R=0.000000,G=1.000000,B=0.000000,A=1.000000)" 2.0))
      (if _returnvalue_2
        (if (not (Math|Boolean|ORBoolean (== (.HitBoneName (Collision|BreakHitResult _outhit)) "head") (== (.HitBoneName (Collision|BreakHitResult _outhit)) "neck_02") (== (.HitBoneName (Collision|BreakHitResult _outhit)) "neck_01")))
          (Class|BPIDamagable|TakeDamage(Message) (.HitActor (Collision|BreakHitResult _outhit)) (Utilities|Struct|MakeS_DamageInfo 25.0 "NewEnumerator2" "NewEnumerator1") self)
          (else
            (Class|BPIDamagable|TakeDamage(Message) (.HitActor (Collision|BreakHitResult _outhit)) (Utilities|Struct|MakeS_DamageInfo 75.0 "NewEnumerator2" "NewEnumerator2") self)))))))

(event EventBeginPlay)

(event Collision|EventActorBeginOverlap
  (params (OtherActor :type Actor%20Object%20Reference)))

(event EventTick
  (params (DeltaSeconds :type Float%20%28single-precision%29)))

(event Input|KeyboardEvents|X
  (params (Key :type Key%20Structure :default "None")))

(fn ConstructionScript
  (|CallParentFunction))
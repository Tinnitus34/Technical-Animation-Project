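; Ranged enemy character that attacks the AI controller's target with a traced hitscan shot from its right hand.
; Attack runs through a server event that fetches the target from AIC_Enemy_Base, then a multicast that plays the montage.
; A montage notify fires a debug-drawn visibility trace, damaging the target only if nothing blocks it; montage end signals attack completion.
; Functions supply walk speeds per movement state and ideal attack and defend ranges.
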(event Custom|ROS_Attack
  ;[0.05098 0.05098 0.05098] Attack Replicated
  (bind _asaic_enemy_base (Utilities|Casting|CastToAIC_Enemy_Base (AI|GetAIController self)))
  (bind _attacktarget (Variables|/Game/TA_Project/Blueprints/Characters/Enemies/IA/AIC_Enemy_Base.AIC_Enemy_Base_C|GetAttackTarget _asaic_enemy_base)
    (:then
      (Variables|Default|SetAttack%20Target _attacktarget)
      (CallFunction|MCAttack))
    (:else)))

(event Custom|MC_Attack
  (bind _attack_target (Variables|Default|GetAttack%20Target))
  ;[0.05098 0.05098 0.05098] Attack Replicated
  (bind _notifyname (Animation|Montage|PlayMontage (Variables|Character|GetMesh) (Variables|Default|GetAttackAnimationMontage))
    (:OnCompleted
      (Default|CallOnAttackEnd :!label _label))
    (:OnInterrupted
      (goto _label))
    (:OnNotifyBegin
      (switch name _notifyname
        (:Fire
          (bind _returnvalue (Collision|LineTraceByChannel (Transformation|GetSocketLocation (Variables|Character|GetMesh) "RightHand") (Transformation|GetActorLocation _attack_target) "TraceTypeQuery1" false 0 "ForDuration"))
          (if (not _returnvalue)
            (Class|BPIDamagable|TakeDamage(Message) _attack_target (Utilities|Struct|MakeS_DamageInfo 2e+01 "NewEnumerator2") self)))))))

(event EventBeginPlay
  (|CallParentFunction))

(event EventAttack
  ;[0.05098 0.05098 0.05098] Attack Replicated
  (CallFunction|ROSAttack))

(fn ConstructionScript
  (|CallParentFunction))

(fn SetMovementSpeed
  (params (Speed :type E_MovementSpeed%20Enum :default "NewEnumerator0"))
  (bind _output_get (Variables|/Script/Engine.CharacterMovementComponent|SetMaxWalkSpeed (Variables|Character|GetCharacterMovement) (Utilities|Select :Index Speed :NewEnumerator0 0.0 :NewEnumerator1 2e+02 :NewEnumerator2 3e+02 :NewEnumerator3 5e+02)))
  (return _output_get))

(fn GetIdealRange
  (return 6e+02 6e+02))
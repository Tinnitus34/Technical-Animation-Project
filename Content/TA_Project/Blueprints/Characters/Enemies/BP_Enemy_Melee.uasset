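; Melee enemy Blueprint that extends a parent enemy class with a close-range attack.
; Attack immediately sphere-traces ahead for pawns with debug drawing and sends a fixed damage struct to the hit actor through a TakeDamage message.
; A montage-driven version, which toggles interruptibility on the damage system and calls OnAttackEnd on completion or interruption, is present but disconnected, so it never runs.
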(event EventBeginPlay
  (|CallParentFunction))

(event EventAttack
  (bind _returnvalue (Transformation|GetActorLocation))
  (bind (_outhit _returnvalue_2) (Collision|SphereTraceForObjects _returnvalue (+ _returnvalue (* (Transformation|GetActorForwardVector) 2e+02)) 2e+01 (Utilities|Array|MakeArray "ObjectTypeQuery3") false 0 "ForDuration"))
  (if _returnvalue_2
    (Class|BPIDamagable|TakeDamage(Message) (.HitActor (Collision|BreakHitResult _outhit)) (Utilities|Struct|MakeS_DamageInfo 25.0 "NewEnumerator1" "NewEnumerator1") self)))

(fn ConstructionScript
  (|CallParentFunction))
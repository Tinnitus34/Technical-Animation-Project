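; Base enemy character that routes health, healing and damage through a damage system component and exposes team, range and movement-speed queries.
; Hits stop movement, play a reaction montage and freeze the AI controller, which switches to attacking after a delay, targeting off-team damage causers.
; Death ragdolls the mesh, disables capsule collision and stops AI logic.
; NavLink jumps launch the character along a suggested projectile arc.
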(event Custom|Die
  (bind _mesh (Variables|Character|GetMesh))
  ;[0.15 0.15 0.15 0.5] Death Event
  (Physics|SetSimulatePhysics _mesh true)
  (Collision|SetCollisionEnabled _mesh "QueryAndPhysics")
  (Collision|SetCollisionEnabled (Variables|Collision|GetCapsuleComponent) "NoCollision")
  (Variables|Default|SetbIsDead true)
  (AI|Logic|StopLogic (Variables|/Script/AIModule.AIController|GetBrainComponent (Variables|Default|GetAICEnemyBase)) "")
  (Default|SetStateasDead (Variables|Default|GetAICEnemyBase))
  (Default|CallOnEnemyDestroyed))

(event Custom|HitResponse
  (params (DamageResponse :type E_DamageResponse%20Enum :default "NewEnumerator0") (NewParam :type E_DamageType%20Enum :default "NewEnumerator0") (DamageCauser :type Actor%20Object%20Reference) (Hit :type Hit%20Result%20Structure))
  ;[0.15 0.15 0.15 0.5] Hit Response
  (Components|Movement|StopMovementImmediately (Variables|Character|GetCharacterMovement))
  (Default|SetStateasFrozen (Variables|Default|GetAICEnemyBase))
  (Animation|Montage|PlayMontage (Variables|Character|GetMesh) (Variables|Default|GetHitReactionMontage)
    (:then
      (bind _teamnumber (Class|BPIDamagable|GetTeamNumber(Message) DamageCauser))
      (Utilities|FlowControl|Delay 1.0)
      (Default|SetStateasAttacking (Variables|Default|GetAICEnemyBase) (select (!= (Variables|Default|GetTeamNumber) _teamnumber) DamageCauser 0) true))))

(event EventBeginPlay
  (bind _bpc_damagesystem (Variables|Default|GetBPC_DamageSystem))
  (Class|SkeletalMeshComponent|SetAllBodiesBelowSimulatePhysics (Variables|Default|GetMesh) (Utilities|Name|MakeLiteralName "pelvis") false false)
  (bind _asaic_enemy_base (Utilities|Casting|CastToAIC_Enemy_Base (AI|GetAIController self)))
  (Variables|Default|SetAICEnemyBase _asaic_enemy_base)
  (EventDispatchers|AssignOnDeath _bpc_damagesystem (EventDispatchers|CreateEvent :!event Custom|Die))
  (EventDispatchers|BindEventtoOnDamageResponse _bpc_damagesystem (EventDispatchers|CreateEvent :!event Custom|HitResponse)))

(event EventJumptoDestination
  (params (Destination :type Vector :default "0, 0, 0"))
  (bind (_x _y _z) (Math|Vector|BreakVector Destination))
  ;[0.05098 0.05098 0.05098] Jump Event With NavLink
  (bind _outlaunchvelocity (Game|SuggestProjectileVelocityCustomArc (Transformation|GetActorLocation) (Math|Vector|MakeVector _x _y (+ _z 2.5e+02)) 0.0 0.5))
  (Character|LaunchCharacter _outlaunchvelocity true true))

(fn ConstructionScript
  (bind _bpc_damagesystem (Variables|Default|GetBPC_DamageSystem))
  (Variables|/Game/TA_Project/Blueprints/Systems/DamageSystem/BPC_DamageSystem.BPC_DamageSystem_C|SetMaxHealth _bpc_damagesystem 1e+02)
  (Variables|/Game/TA_Project/Blueprints/Systems/DamageSystem/BPC_DamageSystem.BPC_DamageSystem_C|SetHealth _bpc_damagesystem 1e+02))

(fn GetActorLocation
  (return "0, 0, 0"))

(fn GetCharacterMesh
  (return (Variables|Character|GetMesh)))

(fn GetCurrentHealth
  (return (Variables|/Game/TA_Project/Blueprints/Systems/DamageSystem/BPC_DamageSystem.BPC_DamageSystem_C|GetHealth (Variables|Default|GetBPC_DamageSystem))))

(fn GetIdealRange
  (return 1.5e+02 3.5e+02))

(fn GetMaxHealth
  (return (Variables|/Game/TA_Project/Blueprints/Systems/DamageSystem/BPC_DamageSystem.BPC_DamageSystem_C|GetMaxHealth (Variables|Default|GetBPC_DamageSystem))))

(fn GetTeamNumber
  (return (Variables|Default|GetTeamNumber)))

(fn Heal
  (params (Amount :type Float%20%28double-precision%29))
  (bind _newhealth (Default|Heal (Variables|Default|GetBPC_DamageSystem) Amount))
  (return _newhealth))

(fn IsDead
  (return (Variables|/Game/TA_Project/Blueprints/Systems/DamageSystem/BPC_DamageSystem.BPC_DamageSystem_C|GetIsDead (Variables|Default|GetBPC_DamageSystem))))

(fn SetMovementSpeed
  (params (Speed :type E_MovementSpeed%20Enum :default "NewEnumerator0"))
  (bind _output_get (Variables|/Script/Engine.CharacterMovementComponent|SetMaxWalkSpeed (Variables|Character|GetCharacterMovement) (Utilities|Select :Index Speed :NewEnumerator0 0.0 :NewEnumerator1 1e+02 :NewEnumerator2 3e+02 :NewEnumerator3 5e+02)))
  (return _output_get))

(fn TakeDamage
  (params (Damage%20Causer :type Actor%20Object%20Reference) (DamageInfo :type S%20Damage%20Info%20Structure) (Hit :type Hit%20Result%20Structure))
  (bind _wasdamaged (Default|TakeDamage (Variables|Default|GetBPC_DamageSystem) DamageInfo Damage%20Causer Hit))
  (return _wasdamaged))
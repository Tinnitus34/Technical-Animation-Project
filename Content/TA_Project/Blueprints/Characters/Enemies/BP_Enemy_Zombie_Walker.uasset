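; Walker zombie enemy that randomizes its skeletal mesh and works with its AI controller to attack and die.
; Attacks play a random montage, blocking interruption, and sphere-trace forward on a notify to deal damage.
; Damage system events trigger physical-animation hit reactions, or death with ragdoll, stopped AI logic and delayed destruction.
; Each tick, walk speed follows an animation root-translation curve; debug healthbar code is disconnected.
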(event Custom|DieZombie
  ;[0.15 0.15 0.15 0.5] Death Event
  (Default|Ragdoll (Variables|Default|GetBPC_PhysicalAnimations))
  (Collision|SetCollisionEnabled (Variables|Character|GetMesh) "QueryAndPhysics")
  (Collision|SetCollisionEnabled (Variables|Default|GetCapsuleComponent) "NoCollision")
  (Variables|Default|SetbIsDead true)
  (AI|Logic|StopLogic (Variables|/Script/AIModule.AIController|GetBrainComponent (Variables|Default|GetRefAICEnemyZombie)) "")
  (Default|SetStateasDead (Variables|Default|GetRefAICEnemyZombie))
  (Default|CallOnEnemyDestroyed)
  (Utilities|FlowControl|Delay 1.2e+02)
  (Actor|DestroyActor))

(event Custom|HitResponseZombie
  (params (DamageResponse :type E_DamageResponse%20Enum :default "NewEnumerator0") (DamageType :type E_DamageType%20Enum :default "NewEnumerator0") (DamageCauser :type Actor%20Object%20Reference) (Hit :type Hit%20Result%20Structure))
  ;[0.15 0.15 0.15 0.5] Hit Response
  (switch Utilities|FlowControl|Switch|SwitchonE_DamageResponse DamageResponse
    (:NewEnumerator1
      (Default|HitReaction (Variables|Default|GetBPC_PhysicalAnimations) Hit))))

(event EventBeginPlay
  (bind _bpc_damagesystem (Variables|Default|GetBPC_DamageSystem))
  (Class|SkeletalMeshComponent|SetAllBodiesBelowSimulatePhysics (Variables|Default|GetMesh) (Utilities|Name|MakeLiteralName "pelvis") false false)
  (Components|SkeletalMesh|SetSkeletalMeshAsset (Variables|Character|GetMesh) (.OutItem (Utilities|Array|Random (Variables|Default|GetListOfMeshes))))
  (bind _asaic_enemy_zombie (Utilities|Casting|CastToAIC_Enemy_Zombie (AI|GetAIController self)))
  (Variables|Default|SetRefAICEnemyZombie _asaic_enemy_zombie)
  (EventDispatchers|AssignOnDeath _bpc_damagesystem (EventDispatchers|CreateEvent :!event Custom|DieZombie))
  (EventDispatchers|BindEventtoOnDamageResponse _bpc_damagesystem (EventDispatchers|CreateEvent :!event Custom|HitResponseZombie)))

(event EventTick
  (params (DeltaSeconds :type Float%20%28single-precision%29))
  (CallFunction|SetSpeed))

(event EventAttack
  (bind _returnvalue (Transformation|GetActorLocation))
  ;[0.15 0.15 0.15 0.5] Attack
  (bind _notifyname (Animation|Montage|PlayMontage (Variables|Character|GetMesh) (.OutItem (Utilities|Array|Random (Variables|Default|GetAttackAnimation))))
    (:then
      (Variables|/Game/TA_Project/Blueprints/Systems/DamageSystem/BPC_DamageSystem.BPC_DamageSystem_C|SetIsinterruptible (Variables|Default|GetBPC_DamageSystem) false))
    (:OnCompleted
      (Default|CallOnAttackEnd :!label _label)
      (Variables|/Game/TA_Project/Blueprints/Systems/DamageSystem/BPC_DamageSystem.BPC_DamageSystem_C|SetIsinterruptible (Variables|Default|GetBPC_DamageSystem) true))
    (:OnInterrupted
      (goto _label))
    (:OnNotifyBegin
      (switch name _notifyname
        (:Attack
          (bind (_outhit _returnvalue_2) (Collision|SphereTraceForObjects _returnvalue (+ _returnvalue (* (Transformation|GetActorForwardVector) 2e+02)) 2e+01 (Utilities|Array|MakeArray "ObjectTypeQuery3") false 0 "ForDuration"))
          (if _returnvalue_2
            (Class|BPIDamagable|TakeDamage(Message) (.HitActor (Collision|BreakHitResult _outhit)) self (Utilities|Struct|MakeS_DamageInfo 1e+01 "NewEnumerator1" "NewEnumerator1"))))))))

(fn ConstructionScript
  (|CallParentFunction))

(fn SetSpeed
  (Variables|/Script/Engine.CharacterMovementComponent|SetMaxWalkSpeed (Variables|Character|GetCharacterMovement) (Math|Float|MapRangeClamped (Animation|Curves|GetCurveValue (Components|SkeletalMesh|GetAnimInstance (Variables|Character|GetMesh)) "root_translation_speed_Y") 2e+01 112.0 53.0 (Variables|/Script/Engine.CharacterMovementComponent|GetMaxWalkSpeed (Variables|Character|GetCharacterMovement)))))
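; Zombie enemy character Blueprint, driven by its AI controller's state changes and a damage system component that triggers its bound events.
; A hit plays a reaction montage and freezes the AI, then after a delay resumes attacking, retargeting non-team damage causers.
; Death ragdolls the mesh, stops AI logic and destroys the actor after a delay.
; Attack applies damage through a forward sphere trace; its montage-driven sequence is disconnected.
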(event Custom|DieZombie
  (bind _mesh (Variables|Character|GetMesh))
  ;[0.15 0.15 0.15 0.5] Death Event
  (Physics|SetSimulatePhysics _mesh true)
  (Collision|SetCollisionEnabled _mesh "QueryAndPhysics")
  (Collision|SetCollisionEnabled (Variables|Default|GetCapsuleComponent) "NoCollision")
  (Variables|Default|SetbIsDead true)
  (AI|Logic|StopLogic (Variables|/Script/AIModule.AIController|GetBrainComponent (Variables|Default|GetRefAICEnemyZombie)) "")
  (Default|SetStateasDead (Variables|Default|GetRefAICEnemyZombie))
  (Default|CallOnEnemyDestroyed)
  (Utilities|FlowControl|Delay 5.0)
  (Actor|DestroyActor))

(event Custom|HitResponseZombie
  (params (DamageResponse :type E_DamageResponse%20Enum :default "NewEnumerator0") (DamageCauser :type Actor%20Object%20Reference))
  ;[0.15 0.15 0.15 0.5] Hit Response
  (Components|Movement|StopMovementImmediately (Variables|Character|GetCharacterMovement))
  (Default|SetStateasFrozen (Variables|Default|GetRefAICEnemyZombie))
  (Animation|Montage|PlayMontage (Variables|Character|GetMesh) (Variables|Default|GetHitReactionAnimation)
    (:then
      (bind _teamnumber (Class|BPIDamagable|GetTeamNumber(Message) DamageCauser))
      (Utilities|FlowControl|Delay 1.0)
      (Default|SetStateasAttacking (Variables|Default|GetRefAICEnemyZombie) (select (!= (Variables|Default|GetTeamNumber) _teamnumber) DamageCauser 0) true))))

(event EventBeginPlay
  (bind _bpc_damagesystem (Variables|Default|GetBPC_DamageSystem))
  (bind _asaic_enemy_zombie (Utilities|Casting|CastToAIC_Enemy_Zombie (AI|GetAIController self)))
  (Variables|Default|SetRefAICEnemyZombie _asaic_enemy_zombie)
  ;[1 1 1 0.5] Healthbar For Debugging
  (bind _returnvalue (UserInterface|CreateWidget "/Game/TA_Project/Blueprints/Systems/DamageSystem/W_Healthbar.W_Healthbar_C" 0 self))
  (UserInterface|SetWidget (Variables|Default|GetHealthbar) _returnvalue)
  (EventDispatchers|AssignOnDeath _bpc_damagesystem (EventDispatchers|CreateEvent :!event Custom|DieZombie))
  (EventDispatchers|BindEventtoOnDamageResponse _bpc_damagesystem (EventDispatchers|CreateEvent :!event Custom|HitResponseZombie)))

(event EventAttack
  (bind _returnvalue (Transformation|GetActorLocation))
  ;[0.15 0.15 0.15 0.5] Attack
  (bind (_outhit _returnvalue_2) (Collision|SphereTraceForObjects _returnvalue (+ _returnvalue (* (Transformation|GetActorForwardVector) 2e+02)) 2e+01 (Utilities|Array|MakeArray "ObjectTypeQuery3") false 0 "ForDuration"))
  (if _returnvalue_2
    (Class|BPIDamagable|TakeDamage(Message) (.HitActor (Collision|BreakHitResult _outhit)) (Utilities|Struct|MakeS_DamageInfo 1e+01 "NewEnumerator1" "NewEnumerator1") self)))

(fn ConstructionScript
  (|CallParentFunction))
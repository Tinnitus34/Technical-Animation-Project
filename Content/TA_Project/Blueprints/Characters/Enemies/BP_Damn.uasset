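; BP_Damn is an enemy character Blueprint whose only custom logic is a long-range, heavy-damage forward attack.
; The Attack event runs a narrow sphere trace for Pawn objects from the actor's location along its forward vector.
; On a hit, it sends a TakeDamage message to the struck actor with an SDamageInfo payload, naming itself as the damage causer.
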(event EventBeginPlay
  (|CallParentFunction) ; This node is disabled and will not be called.\nDrag off pins to build functionality.
)

(event Collision|EventActorBeginOverlap
  (params (OtherActor :type Actor%20Object%20Reference)))

(event EventTick
  (params (DeltaSeconds :type Float%20%28single-precision%29)))

(event EventAttack
  (bind _returnvalue (Transformation|GetActorLocation))
  (bind (_outhit _returnvalue_2) (Collision|SphereTraceForObjects _returnvalue (+ _returnvalue (* (Transformation|GetActorForwardVector) 5e+03)) 2e+01 (Utilities|Array|MakeArray "ObjectTypeQuery3") false 0 "None"))
  (if _returnvalue_2
    (Class|BPIDamagable|TakeDamage(Message) (.HitActor (Collision|BreakHitResult _outhit)) self (Utilities|Struct|MakeS_DamageInfo 5e+02 "NewEnumerator1" "NewEnumerator1" true))))

(fn ConstructionScript
  (|CallParentFunction))
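; BP_AmmoBox is an interactable ammo box that presents a "TO TAKE AMMO" prompt.
; It supplies interaction location from a component, along with prompt, type, hold duration and tap count, through getter functions.
; Interact loops over every BP_WeaponBase actor, but the loop body is empty and the carried-ammo message call is disconnected, so no ammo is granted.
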(event EventBeginPlay
  (|CallParentFunction) ; This node is disabled and will not be called.\nDrag off pins to build functionality.
)

(event Collision|EventActorBeginOverlap
  (params (OtherActor :type Actor%20Object%20Reference))
  (|CallParentFunction OtherActor) ; This node is disabled and will not be called.\nDrag off pins to build functionality.
)

(event EventTick
  (params (DeltaSeconds :type Float%20%28single-precision%29))
  (|CallParentFunction DeltaSeconds) ; This node is disabled and will not be called.\nDrag off pins to build functionality.
)

(event EventInteract
  (params (Interactor :type Actor%20Object%20Reference))
  (bind _outactors (Actor|GetAllActorsOfClass "/Game/TA_Project/Blueprints/Systems/WeaponSystem/Weapons/BP_WeaponBase.BP_WeaponBase_C"))
  (for _array_element _outactors
    _))

(fn ConstructionScript
  (|CallParentFunction))

(fn GetInteractionLocation
  (return (Transformation|GetWorldLocation (Variables|Default|GetInteractionLocation))))

(fn GetInteractionPrompt
  (return "TO TAKE AMMO"))

(fn GetInteractionType
  (return "NewEnumerator0"))

(fn GetHoldDuration
  (return 0.0))

(fn GetTapCount
  (return 0))
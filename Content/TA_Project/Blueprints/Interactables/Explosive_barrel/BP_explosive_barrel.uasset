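; Explosive barrel interactable that explodes when its damage component reports a damage response, rather than on death, which is left empty.
; BPCDamageSystem handles incoming damage and health queries, with getters subtracting a fixed offset, while healing does nothing.
; The blast spawns effects and sound, activates RadialForce, damages pawns found by a sphere trace of that force's radius, then destroys the barrel after a short delay.
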(event Custom|Death)

(event Custom|DamageResponse
  (params (DamageResponse :type E_DamageResponse%20Enum :default "NewEnumerator0") (DamageType :type E_DamageType%20Enum :default "NewEnumerator0") (Causer :type Actor%20Object%20Reference) (Hit :type Hit%20Result%20Structure))
  (bind _returnvalue (Transformation|GetActorLocation))
  (bind _returnvalue_2 (Transformation|GetActorLocation))
  (bind _radialforce (Variables|Default|GetRadialForce))
  ;[0.15 0.15 0.15 0.5] Explosion effect
  (Effects|SpawnEmitteratLocation "/Game/TA_Project/StarterContent/Particles/P_Explosion.P_Explosion" _returnvalue (Math|Conversions|RotationFromXVector _returnvalue) "2.000000,2.000000,1.000000")
  (Audio|SpawnSoundatLocation "/Game/TA_Project/StarterContent/Audio/Explosion02.Explosion02" (Transformation|GetActorLocation self) "0, 0, 0" 0.5 (Math|Random|RandomFloatinRange 0.9 1.1) 0.0 0 0)
  (Components|Activation|SetActive _radialforce true false)
  (bind (_outhits _returnvalue_3) (Collision|MultiSphereTraceForObjects _returnvalue_2 _returnvalue_2 (Variables|/Script/Engine.RadialForceComponent|GetRadius _radialforce) (Utilities|Array|MakeArray "ObjectTypeQuery3") false 0 "None"))
  (Utilities|FlowControl|Sequence
    (:then_0
      (if _returnvalue_3
        (for _array_element _outhits
          (Class|BPIDamagable|TakeDamage(Message) (.HitActor (Collision|BreakHitResult _array_element)) self (Utilities|Struct|MakeS_DamageInfo 8e+01 "NewEnumerator3" "NewEnumerator4")))))
    (:then_1
      (Utilities|FlowControl|Delay 0.2)
      (Actor|DestroyActor))))

(event EventBeginPlay)

(event Collision|EventActorBeginOverlap
  (params (OtherActor :type Actor%20Object%20Reference)))

(event EventTick
  (params (DeltaSeconds :type Float%20%28single-precision%29)))

(fn ConstructionScript
  (bind _bpc_damagesystem (Variables|Components|GetBPC_DamageSystem))
  (EventDispatchers|BindEventtoOnDeath _bpc_damagesystem (EventDispatchers|CreateEvent :!event Custom|Death))
  (EventDispatchers|BindEventtoOnDamageResponse _bpc_damagesystem (EventDispatchers|CreateEvent :!event Custom|DamageResponse)))

(fn GetCurrentHealth
  (return (- (Variables|/Game/TA_Project/Blueprints/Systems/DamageSystem/BPC_DamageSystem.BPC_DamageSystem_C|GetHealth (Variables|Components|GetBPC_DamageSystem)) 75.0)))

(fn GetMaxHealth
  (return (- (Variables|/Game/TA_Project/Blueprints/Systems/DamageSystem/BPC_DamageSystem.BPC_DamageSystem_C|GetMaxHealth (Variables|Components|GetBPC_DamageSystem)) 75.0)))

(fn GetTeamNumber
  (return 0))

(fn Heal
  (params (Amount :type Float%20%28double-precision%29))
  (return 0.0))

(fn IsDead
  (return (Variables|/Game/TA_Project/Blueprints/Systems/DamageSystem/BPC_DamageSystem.BPC_DamageSystem_C|GetIsDead (Variables|Components|GetBPC_DamageSystem))))

(fn TakeDamage
  (params (Damage%20Causer :type Actor%20Object%20Reference) (DamageInfo :type S%20Damage%20Info%20Structure) (Hit :type Hit%20Result%20Structure))
  (bind _wasdamaged (Default|TakeDamage (Variables|Components|GetBPC_DamageSystem) DamageInfo Damage%20Causer))
  (return _wasdamaged))
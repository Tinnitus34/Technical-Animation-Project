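; Wave-system enemy spawner actor that holds a queue of enemy classes and spawns them at its own transform.
; Queued enemies spawn immediately if no enemy overlaps its sphere, while a looping timer drives further spawn attempts.
; It binds to each spawned enemy's destruction to report defeats to the game mode.
; When the wave component ends a wave, it sets IsOn by comparing the next wave number to its activation round.
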(event Custom|TryToSpawn
  (CallFunction|SpawnEnemy))

(event Custom|OnEnemyDefeated
  (Class|BPIWaveEnemySystem|CallonEnemyDefeated(Message) (Game|GetGameMode)))

(event Custom|OnEndWave
  (Variables|Default|SetIsOn (>= (+ (Variables|/Game/TA_Project/Blueprints/Systems/EnemyWaveSystem/WaveEnemySystem.WaveEnemySystem_C|GetWaveNumber (Variables|Default|GetRefWaveEnemyComponent)) 1) (Variables|Default|GetRoundActivated))))

(event EventBeginPlay
  (Utilities|Time|SetTimerbyEvent (EventDispatchers|CreateEvent :!event Custom|TryToSpawn) 2.0 true)
  (bind _waveenemycomponent (Class|BPIWaveEnemySystem|GetWaveEnemyComponent(Message) (Game|GetGameMode)))
  (bind _output_get (Variables|Default|SetRefWaveEnemyComponent _waveenemycomponent))
  (EventDispatchers|BindEventtoOnEndWave _output_get (EventDispatchers|CreateEvent :!event Custom|OnEndWave)))

(fn ConstructionScript)

(fn SpawnEnemy
  (if (Utilities|Array|IsValidIndex (Variables|Default|GetEnemyQueue))
    (bind _returnvalue (Game|SpawnActorfromClass (Utilities|Array|Get(acopy) (Variables|Default|GetEnemyQueue)) (Transformation|GetActorTransform) "AdjustIfPossibleButAlwaysSpawn" "MultiplyWithRoot" 0 1 0))
    (EventDispatchers|BindEventtoOnEnemyDestroyed _returnvalue (EventDispatchers|CreateEvent :!event Custom|OnEnemyDefeated))
    (Utilities|Array|RemoveIndex (Variables|Default|GetEnemyQueue))
    (return true)
    (else
      (return false))))

(fn AddEnemytoQueue
  (params (EnemyClass :type BP%20Enemy%20Base%20Class%20Reference%20%28by%20ref%29))
  (Utilities|Array|Add (Variables|Default|GetEnemyQueue) EnemyClass)
  (if (not (Utilities|Array|IsValidIndex (Collision|GetOverlappingActors (Variables|Default|GetSphere) "/Game/TA_Project/Blueprints/Characters/Enemies/BP_Enemy_Base.BP_Enemy_Base_C" :!class /Script/Engine.PrimitiveComponent)))
    (CallFunction|SpawnEnemy)))
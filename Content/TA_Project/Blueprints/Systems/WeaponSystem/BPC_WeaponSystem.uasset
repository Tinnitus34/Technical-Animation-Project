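; Weapon system component for the player character, handling shooting, reloading, ammo refills and swapping between socket-attached weapons.
; Weapon stats, montages and sounds load from a data table; switching unequips the previous weapon before equipping the next.
; Montage notifies time socket attachment, reloading and the camera line-trace shot, which multiplies damage on head or neck bones.
; Ammo lives on weapon actors, found by GetActorOfClass and accessed through message calls.
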(event EventBeginPlay
  (EventDispatchers|BindEventtoOnNewAction (EventDispatchers|CreateEvent :!event ManageAction))
  (EventDispatchers|BindEventtoOnChangingDatas (EventDispatchers|CreateEvent :!event SetPreviousData)))

(event EventTick
  (params (DeltaSeconds :type Float%20%28single-precision%29)))

(event Custom|Reload
  ;[1 1 1] Reload Action
  (if (PureFunction|CanReload)
    (Utilities|FlowControl|DoOnce false :!label _label
      (:Completed
        (bind _notifyname (Animation|Montage|PlayMontage (PureFunction|GetCharacterMesh) (Variables|Montages|GetReloadMontage))
          (:then
            (Audio|PlaySound2D (Variables|Sounds|GetReloadSound) 0.6 (Math|Random|RandomFloatinRange 0.9 1.1) 0.0 0 0))
          (:OnCompleted
            (goto _label Reset))
          (:OnInterrupted
            (goto _label Reset))
          (:OnNotifyBegin
            (switch name _notifyname
              (:Reload
                (CallFunction|ReloadLogic)))))))))

(event Custom|Equip
  (params (MontageToPlay :type Anim%20Montage%20Object%20Reference) (SocketName :type Name) (AnimationType :type E_ActionType%20Enum :default "NewEnumerator0"))
  ;[1 1 1] Equip Action
  (bind _notifyname (Animation|Montage|PlayMontage (PureFunction|GetCharacterMesh) MontageToPlay)
    (:OnNotifyBegin
      (switch name _notifyname
        (:Attach
          (CallFunction|AttachWeapon SocketName AnimationType))))))

(event Custom|Shoot
  ;[1 1 1] Shoot Action
  (if (and (PureFunction|IsAiming) (PureFunction|CanShoot))
    (if (not (PureFunction|IsMontagePlaying))
      (Utilities|FlowControl|DoOnce false :!label _label
        (:Completed
          (bind _notifyname (Animation|Montage|PlayMontage (PureFunction|GetCharacterMesh) (Variables|Montages|GetRecoilMontage) 0.5)
            (:then
              (Audio|PlaySound2D (Variables|Sounds|GetShootSound) 0.6 (Math|Random|RandomFloatinRange 0.9 1.1) 0.1 0 0))
            (:OnCompleted
              (goto _label Reset))
            (:OnInterrupted
              (goto _label Reset))
            (:OnNotifyBegin
              (switch name _notifyname
                (:Shoot
                  (CallFunction|ShootLogic))))))))
    (else
      (Audio|PlaySound2D (Variables|Sounds|GetEmptySound) 0.6 (Math|Random|RandomFloatinRange 0.9 1.1) 0.0 0 0))))

(event Custom|Unequip
  (params (MontageToPlay :type Anim%20Montage%20Object%20Reference) (SocketName :type Name) (AnimationType :type E_ActionType%20Enum :default "NewEnumerator0"))
  ;[1 1 1] Unequip Action
  (bind _notifyname (Animation|Montage|PlayMontage (PureFunction|GetCharacterMesh) MontageToPlay)
    (:OnCompleted
      _)
    (:OnNotifyBegin
      (switch name _notifyname
        (:Attach
          (CallFunction|AttachWeapon SocketName AnimationType)))))
  (Default|CallOnChangingDatas)
  (Default|CallOnNewAction "NewEnumerator2"))

(fn EquipWeapon
  (params (WeaponID :type Integer))
  ;[1 1 1] Equip Weapon (Set current weapon details and then switch to it)
  (CallFunction|SetWeaponDetails WeaponID)
  (bind _weapontype (CallFunction|SwitchWeapon))
  (return _weapontype))

(fn SetWeaponDetails
  (params (WeaponID :type Integer))
  ;[1 1 1] Set all details of the current weapon from the data table.
  (bind _output_get (Variables|Default|SetWeaponID WeaponID))
  (bind _returnvalue (Utilities|GetDataTableRow "/Game/TA_Project/Blueprints/Systems/WeaponSystem/WeaponPoolTable.WeaponPoolTable" (Utilities|String|StringToName (Utilities|String|ToString(Integer) _output_get)))
    (:then
      (|SetVariables (.Weapon (Utilities|Struct|BreakFWeaponStruct _returnvalue)) (.WeaponName (Utilities|Struct|BreakFWeaponStruct _returnvalue)) (.EquippedSocketName (Utilities|Struct|BreakFWeaponStruct _returnvalue)) (.UnequippedSocketName (Utilities|Struct|BreakFWeaponStruct _returnvalue)) (.MaxAmmo (Utilities|Struct|BreakFWeaponStruct _returnvalue)) (.MaxCarriedAmmo (Utilities|Struct|BreakFWeaponStruct _returnvalue)) (.Damage (Utilities|Struct|BreakFWeaponStruct _returnvalue)) (.HeadshotMultiplier (Utilities|Struct|BreakFWeaponStruct _returnvalue)) (.RecoilMontage (Utilities|Struct|BreakFWeaponStruct _returnvalue)) (.ReloadMontage (Utilities|Struct|BreakFWeaponStruct _returnvalue)) (.EquipMontage (Utilities|Struct|BreakFWeaponStruct _returnvalue)) (.ShootSound (Utilities|Struct|BreakFWeaponStruct _returnvalue)) (.EmptySound (Utilities|Struct|BreakFWeaponStruct _returnvalue)) (.ReloadSound (Utilities|Struct|BreakFWeaponStruct _returnvalue)) (.ShootParticle (Utilities|Struct|BreakFWeaponStruct _returnvalue))))))

(fn SwitchWeapon
  (if (not (== (Variables|Default|GetWeapon) (Variables|Default|GetPreviousWeapon)))
    ;[1 1 1] If previous weapon is set (a weapon is already equipped), unequip first.
    (Variables|Default|GetPreviousWeapon
      (:then
        (CallFunction|ManageAction "NewEnumerator1"))
      (:else
        (CallFunction|ManageAction "NewEnumerator2")
        (CallFunction|SetPreviousData)))
    (return (Variables|Default|GetWeaponList))
    (else
      ;[1 1 1] Do not switch if already equipped.
      (return (Variables|Default|GetPreviousWeaponList)))))

(fn AttachNewWeapon
  (params (Character :type Character%20Object%20Reference) (WeaponID :type Integer))
  ;[1 1 1] Attach initial weapons to their Unequipped socket.
  (Utilities|Array|AddUnique (Variables|Default|GetEquippedWeapons) WeaponID)
  (CallFunction|SetWeaponDetails WeaponID)
  (bind _returnvalue (Game|SpawnActorfromClass (Variables|Default|GetWeapon) (Math|Transform|MakeTransform "0, 0, 0" "0, 0, 0" "1.000000,1.000000,1.000000") "AlwaysSpawn" "MultiplyWithRoot" 0 0))
  (Transformation|AttachComponentToComponent (Variables|/Script/Engine.Actor|GetRootComponent _returnvalue) (Variables|/Script/Engine.Character|GetMesh Character) (Variables|Sockets|GetUnequippedSocketName) "KeepRelative" "KeepRelative" "KeepRelative" true))

(fn AttachWeapon
  (params (SocketName :type Name) (AnimationType :type E_ActionType%20Enum :default "NewEnumerator0"))
  ;[1 1 1] Attach Weapon to unequipped socket and equipped socket based on enumerator.
  (bind _returnvalue (Actor|GetActorOfClass (Utilities|Select :Index AnimationType :NewEnumerator2 (Variables|Default|GetWeapon) :NewEnumerator1 (Variables|Default|GetPreviousWeapon))))
  (Transformation|AttachComponentToComponent (Variables|/Script/Engine.Actor|GetRootComponent _returnvalue) (Variables|/Script/Engine.Character|GetMesh (Game|GetPlayerCharacter 0)) SocketName "KeepRelative" "KeepRelative" "KeepRelative" true)
  (return))

(fn CanShoot
  (bind _ammo (Class|BPIWeaponSystemWeapons|GetAmmo(Message) (PureFunction|GetWeaponRef)))
  (return (> _ammo 0)))

(fn CanReload
  (bind (_ammo _carriedammo) (PureFunction|GetAmmoValues))
  (return (and (< _ammo (Variables|Default|GetMaxAmmo)) (> _carriedammo 0))))

(fn IsAiming
  (bind _isaiming (Class|BPIWeaponSystemCharacter|GetIsAiming(Message) (Game|GetPlayerCharacter 0)))
  (return _isaiming))

(fn RefillAllAmmo
  ;[1 1 1] Refill all ammo if missing atleast 1.
  (for _array_element (Variables|Default|GetEquippedWeapons)
    (bind _returnvalue (Utilities|GetDataTableRow "/Game/TA_Project/Blueprints/Systems/WeaponSystem/WeaponPoolTable.WeaponPoolTable" (Utilities|String|StringToName (Utilities|String|ToString(Integer) _array_element)))
      (:then
        (bind _returnvalue_2 (Actor|GetActorOfClass (.Weapon (Utilities|Struct|BreakFWeaponStruct _returnvalue))))
        (bind _ammo (Class|BPIWeaponSystemWeapons|GetAmmo(Message) _returnvalue_2))
        (bind _carriedammo (Class|BPIWeaponSystemWeapons|GetCarriedAmmo(Message) _returnvalue_2))
        (if (or (< _ammo (.MaxAmmo (Utilities|Struct|BreakFWeaponStruct _returnvalue))) (< _carriedammo (.MaxCarriedAmmo (Utilities|Struct|BreakFWeaponStruct _returnvalue))))
          (Utilities|FlowControl|Sequence
            (:then_0
              (Utilities|FlowControl|DoOnce false
                (:Completed
                  (LocalVariables|SetLocalCanRefill true))))
            (:then_1
              (Class|BPIWeaponSystemWeapons|SetAmmo(Message) _returnvalue_2 (.MaxAmmo (Utilities|Struct|BreakFWeaponStruct _returnvalue)))
              (Class|BPIWeaponSystemWeapons|SetCarriedAmmo(Message) _returnvalue_2 (.MaxCarriedAmmo (Utilities|Struct|BreakFWeaponStruct _returnvalue)))))))))
  (if (LocalVariables|GetLocalCanRefill)
    (return true)
    (else
      (return false))))

(fn ReloadLogic
  (bind (_ammo _carriedammo) (PureFunction|GetAmmoValues))
  ;[1 1 1] Reload Logic
  (LocalVariables|SetWeaponREF (PureFunction|GetWeaponRef))
  (LocalVariables|SetCarriedAmmo _carriedammo)
  (LocalVariables|SetAmmo _ammo)
  (if (>= (LocalVariables|GetCarriedAmmo) (- (Variables|Default|GetMaxAmmo) (LocalVariables|GetAmmo)))
    (Class|BPIWeaponSystemWeapons|SetCarriedAmmo(Message) (LocalVariables|GetWeaponREF) (- (LocalVariables|GetCarriedAmmo) (- (Variables|Default|GetMaxAmmo) (LocalVariables|GetAmmo))))
    (Class|BPIWeaponSystemWeapons|SetAmmo(Message) (LocalVariables|GetWeaponREF) (Variables|Default|GetMaxAmmo))
    (else
      (Class|BPIWeaponSystemWeapons|SetCarriedAmmo(Message) (LocalVariables|GetWeaponREF))
      (Class|BPIWeaponSystemWeapons|SetAmmo(Message) (LocalVariables|GetWeaponREF) (+ (LocalVariables|GetAmmo) (LocalVariables|GetCarriedAmmo))))))

(fn ShootLogic
  (bind _skeletalmesh (PureFunction|GetWeaponSkeletalMesh))
  (bind _camera (PureFunction|GetCameraRef))
  (bind _returnvalue (Transformation|GetWorldLocation _camera))
  (bind _returnvalue_2 (Transformation|GetSocketTransform _skeletalmesh "muzzle" "RTS_World"))
  (Effects|SpawnEmitterAttached (Variables|Default|GetShootParticle) _skeletalmesh "muzzle" (+ (.location _returnvalue_2) (* (Math|Vector|GetForwardVector (.rotation _returnvalue_2)) 15.0)) (.rotation _returnvalue_2) "0.050000,0.050000,0.050000" "KeepWorldPosition")
  (bind (_outhit _returnvalue_3) (Collision|LineTraceByChannel _returnvalue (+ _returnvalue (* (Math|Vector|GetForwardVector _camera) 5e+03)) "TraceTypeQuery1" false 0 "None" true "(R=1.000000,G=0.000000,B=0.000000,A=1.000000)" "(R=0.000000,G=1.000000,B=0.000000,A=1.000000)" 2.0))
  (CallFunction|RemoveBullet)
  (if _returnvalue_3
    (if (not (Math|Boolean|ORBoolean (== (.HitBoneName (Collision|BreakHitResult _outhit)) "head") (== (.HitBoneName (Collision|BreakHitResult _outhit)) "neck_02") (== (.HitBoneName (Collision|BreakHitResult _outhit)) "neck_01")))
      (Class|BPIDamagable|TakeDamage(Message) (.HitActor (Collision|BreakHitResult _outhit)) (Game|GetPlayerCharacter 0) (Utilities|Struct|MakeS_DamageInfo (Variables|Default|GetDamage) "NewEnumerator2" "NewEnumerator1") _outhit)
      (else
        (Class|BPIDamagable|TakeDamage(Message) (.HitActor (Collision|BreakHitResult _outhit)) (Game|GetPlayerCharacter 0) (Utilities|Struct|MakeS_DamageInfo (* (Variables|Default|GetDamage) (Variables|Default|GetHeadshotMult)) "NewEnumerator2" "NewEnumerator1") _outhit)))))

(fn ManageAction
  (params (Animation%20Type :type E_ActionType%20Enum :default "NewEnumerator0"))
  (bind _output_get (LocalVariables|SetAnimationType Animation%20Type))
  (switch Utilities|FlowControl|Switch|SwitchonE_ActionType _output_get
    (:NewEnumerator2
      (CallFunction|Equip (Utilities|Select :Index (LocalVariables|GetAnimationType) :NewEnumerator2 (Variables|Montages|GetEquipUnequipMontage) :NewEnumerator1 (Variables|Montages|GetPreviousEquipUnequipMontage)) (Utilities|Select :Index (LocalVariables|GetAnimationType) :NewEnumerator2 (Variables|Sockets|GetEquippedSocketName) :NewEnumerator1 (Variables|Sockets|GetPrevousUnequippedSocketName)) (LocalVariables|GetAnimationType)))
    (:NewEnumerator1
      (CallFunction|Unequip (Utilities|Select :Index (LocalVariables|GetAnimationType) :NewEnumerator2 (Variables|Montages|GetEquipUnequipMontage) :NewEnumerator1 (Variables|Montages|GetPreviousEquipUnequipMontage)) (Utilities|Select :Index (LocalVariables|GetAnimationType) :NewEnumerator2 (Variables|Sockets|GetEquippedSocketName) :NewEnumerator1 (Variables|Sockets|GetPrevousUnequippedSocketName)) (LocalVariables|GetAnimationType)))))

(fn GetAmmoValues
  (bind _weapon (PureFunction|GetWeaponRef))
  (bind _ammo (Class|BPIWeaponSystemWeapons|GetAmmo(Message) _weapon))
  (bind _carriedammo (Class|BPIWeaponSystemWeapons|GetCarriedAmmo(Message) _weapon))
  (return _ammo _carriedammo))

(fn GetWeaponRef
  (bind _returnvalue (Actor|GetActorOfClass (Variables|Default|GetWeapon)))
  (return _returnvalue))

(fn SetPreviousData
  (Variables|Default|SetPreviousWeapon (Variables|Default|GetWeapon))
  (Variables|Montages|SetPreviousEquipUnequipMontage (Variables|Montages|GetEquipUnequipMontage))
  (Variables|Sockets|SetPrevousUnequippedSocketName (Variables|Sockets|GetUnequippedSocketName))
  (Variables|Default|SetPreviousWeaponList (Variables|Default|GetWeaponList)))

(fn GetWeaponLocation
  (bind _returnvalue (Actor|GetActorOfClass (Variables|Default|GetWeapon)))
  (return (Transformation|GetSocketTransform (Variables|/Game/TA_Project/Blueprints/Systems/WeaponSystem/Weapons/BP_WeaponBase.BP_WeaponBase_C|GetSkeletalMesh _returnvalue) "equip2" "RTS_World")))

(fn GetCharacterMesh
  (return (Variables|/Script/Engine.Character|GetMesh (Game|GetPlayerCharacter 0))))

(fn IsMontagePlaying
  (return (Class|AnimInstance|IsAnyMontagePlaying (Components|SkeletalMesh|GetAnimInstance (PureFunction|GetCharacterMesh)))))

(fn GetWeaponSkeletalMesh
  (return (Variables|/Game/TA_Project/Blueprints/Systems/WeaponSystem/Weapons/BP_WeaponBase.BP_WeaponBase_C|GetSkeletalMesh (PureFunction|GetWeaponRef))))

(fn GetCameraRef
  (bind _newparam (Class|BPIWeaponSystemCharacter|GetCameraRef(Message) (Game|GetPlayerCharacter 0)))
  (return _newparam))

(fn RemoveBullet
  (Class|BPIWeaponSystemWeapons|SetAmmo(Message) (PureFunction|GetWeaponRef) (- (.Ammo (PureFunction|GetAmmoValues)) 1)))
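; Revolver weapon in the weapon system that fires hitscan shots and tracks loaded and carried ammo.
; When allowed, Shoot plays a sound, decrements ammo and line-traces from the camera with debug drawing.
; Hits send a damage message, with head and neck bones taking higher hardcoded damage independent of the Damage variable.
; Accessor functions expose both ammo counts for read and write, and Damage as read-only.
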(event EventBeginPlay
  (|CallParentFunction))

(event Collision|EventActorBeginOverlap
  (params (OtherActor :type Actor%20Object%20Reference))
  (|CallParentFunction OtherActor) ; This node is disabled and will not be called.\nDrag off pins to build functionality.
)

(event EventTick
  (params (DeltaSeconds :type Float%20%28single-precision%29))
  (|CallParentFunction DeltaSeconds) ; This node is disabled and will not be called.\nDrag off pins to build functionality.
)

(event EventShoot
  (params (CanShoot :type Boolean))
  (bind _camera (Variables|Default|GetCamera))
  (bind _returnvalue (Transformation|GetWorldLocation _camera))
  (if CanShoot
    (Audio|PlaySound2D "/Game/TA_Project/Sounds/SoundEffects/RevolverShootSound.RevolverShootSound" 0.3 1.0 0.0 0 0)
    (bind (_outhit _returnvalue_2) (Collision|LineTraceByChannel _returnvalue (+ _returnvalue (* (Math|Vector|GetForwardVector _camera) 5e+03)) "TraceTypeQuery1" false 0 "ForDuration" true "(R=1.000000,G=0.000000,B=0.000000,A=1.000000)" "(R=0.000000,G=1.000000,B=0.000000,A=1.000000)" 2.0))
    (Math|Integer|DecrementInt (Variables|Default|GetAmmo)
      (:%20%20
        (if _returnvalue_2
          (if (not (Math|Boolean|ORBoolean (== (.HitBoneName (Collision|BreakHitResult _outhit)) "head") (== (.HitBoneName (Collision|BreakHitResult _outhit)) "neck_02") (== (.HitBoneName (Collision|BreakHitResult _outhit)) "neck_01")))
            (Class|BPIDamagable|TakeDamage(Message) (.HitActor (Collision|BreakHitResult _outhit)) (Utilities|Struct|MakeS_DamageInfo 25.0 "NewEnumerator2" "NewEnumerator1") (Variables|Default|GetCharacter))
            (else
              (Class|BPIDamagable|TakeDamage(Message) (.HitActor (Collision|BreakHitResult _outhit)) (Utilities|Struct|MakeS_DamageInfo 75.0 "NewEnumerator2" "NewEnumerator2") (Variables|Default|GetCharacter)))))))))

(fn ConstructionScript
  (|CallParentFunction))

(fn GetAmmo
  (return (Variables|Default|GetAmmo)))

(fn GetCarriedAmmo
  (return (Variables|Default|GetCarriedAmmo)))

(fn GetDamage
  (return (Variables|Default|GetDamage)))

(fn SetAmmo
  (params (NewAmmo :type Integer))
  (Variables|Default|SetAmmo NewAmmo)
  (return true))

(fn SetCarriedAmmo
  (params (NewCarriedAmmo :type Integer))
  (Variables|Default|SetCarriedAmmo NewCarriedAmmo)
  (return true))
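; BP_WeaponBase is a weapon base Blueprint that holds ammo state and references to the player character and its camera.
; On BeginPlay, SetRef finds BP_Core_Character with GetActorOfClass, then caches the camera returned by its GetCameraRefMessage call.
; Simple getters and setters expose loaded and carried ammo, with setters always returning true and applying no validation.
; The file contains no firing or reload logic.
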(event EventBeginPlay
  (CallFunction|SetRef))

(fn ConstructionScript)

(fn SetRef
  (bind _returnvalue (Actor|GetActorOfClass "/Game/TA_Project/Blueprints/Gamemode/Core/BP_Core_Character.BP_Core_Character_C"))
  (bind _output_get (Variables|Default|SetCharacter _returnvalue))
  (bind _newparam (Class|BPIWeaponSystemCharacter|GetCameraRef(Message) _output_get))
  (Variables|Default|SetCamera _newparam))

(fn GetAmmo
  (return (Variables|Default|GetAmmo)))

(fn GetCarriedAmmo
  (return (Variables|Default|GetCarriedAmmo)))

(fn SetAmmo
  (params (NewAmmo :type Integer))
  (Variables|Default|SetAmmo NewAmmo)
  (return true))

(fn SetCarriedAmmo
  (params (NewCarriedAmmo :type Integer))
  (Variables|Default|SetCarriedAmmo NewCarriedAmmo)
  (return true))
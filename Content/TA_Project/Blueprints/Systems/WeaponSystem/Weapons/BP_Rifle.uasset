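; BP_Rifle is the rifle Blueprint in the weapon system, holding the weapon's loaded and carried ammo counts.
; Simple getters and setters expose Ammo and CarriedAmmo, with both setters storing the value unvalidated and always returning true.
; GetDamage is a stub that returns zero.
; It has no firing or reload logic of its own, its event graph is disabled, and construction only calls the parent.
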(event EventBeginPlay
  (|CallParentFunction) ; This node is disabled and will not be called.\nDrag off pins to build functionality.
)

(event Collision|EventActorBeginOverlap
  (params (OtherActor :type Actor%20Object%20Reference))
  (|CallParentFunction OtherActor) ; This node is disabled and will not be called.\nDrag off pins to build functionality.
)

(event EventTick
  (params (DeltaSeconds :type Float%20%28single-precision%29))
  (|CallParentFunction DeltaSeconds) ; This node is disabled and will not be called.\nDrag off pins to build functionality.
)

(fn ConstructionScript
  (|CallParentFunction))

(fn GetCarriedAmmo
  (return (Variables|Default|GetCarriedAmmo)))

(fn GetAmmo
  (return (Variables|Default|GetAmmo)))

(fn SetCarriedAmmo
  (params (NewCarriedAmmo :type Integer))
  (Variables|Default|SetCarriedAmmo NewCarriedAmmo)
  (return true))

(fn SetAmmo
  (params (NewAmmo :type Integer))
  (Variables|Default|SetAmmo NewAmmo)
  (return true))

(fn GetDamage
  (return 0.0))